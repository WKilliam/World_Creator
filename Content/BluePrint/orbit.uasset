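; Actor Blueprint that moves itself in a horizontal circular path, with configurable speed, direction, radius and angle offset.
; Tick accumulates a rotation angle and passes it to RotationDeActeur, which rotates a radius vector around Z and adds it to the actor's location.
; Because that location is the actor's current one, steps accumulate each frame, leaving the stored start location and target actor effectively unused.
; Optional debug lines trace each step.
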(event `self.ReceiveBeginPlay`
  (set `self.InitialisationLocation` (`self.K2_GetActorLocation`)))

(event `self.ReceiveTick`
  (params (DeltaSeconds :type "Float (single-precision)"))
  (set `self.CurrentRotation` (+ (`self.CurrentRotation`) (* (* (`self.Vitesse_Rotation`) DeltaSeconds) (`KismetMathLibrary.SelectFloat` 1.0 -1.0 (`self.Sens_Aiguilles`)))))
  (bind _newparam (`self.Rotation_De_Acteur` self (`self.CibleActor`) (`self.InitialisationLocation`) (`self.Radius`) (`self.Angle`) (`self.CurrentRotation`)))
  (if (`self.Debug`)
    (`KismetSystemLibrary.DrawDebugLine` _newparam (`self.K2_GetActorLocation`) (`self.Trace_Color`) 1.0 2.0)))

(fn `Rotation_De_Acteur`
  (params (Acteur_de_rotation :type "Actor Object Reference") (Acteur_cible :type "Actor Object Reference") (Location_cidle :type "Vector Structure") (Radian :type "Float (double-precision)") (Angle :type "Float (double-precision)") (Rotation_pourcentage :type "Float (double-precision)"))
  (returns (NewParam :type "Vector Structure"))
  (locals (FLActor_Rotation :type "Actor Object Reference") (FCible_Acteur :type "Actor Object Reference") (NewLocalVar_2 :type "Vector Structure") (NewLocalVar_3 :type "Float (double-precision)") (NewLocalVar_4 :type "Float (double-precision)") (NewLocalVar_5 :type "Float (double-precision)") (FLacation :type "Vector Structure") (FRadian :type "Float (double-precision)") (FAngle :type "Float (double-precision)") (FTaux :type "Float (double-precision)"))
  (set `local.FLActor_Rotation` Acteur_de_rotation)
  (set `local.FCible_Acteur` Acteur_cible)
  (set `local.FLacation` Location_cidle)
  (set `local.FRadian` Radian)
  (set `local.FAngle` Angle)
  (set `local.FTaux` Rotation_pourcentage)
  (`/Engine/EditorBlueprintResources/StandardMacros.IsValid` (`local.FLActor_Rotation`)
    (:`Is Valid`
      (set `local.FLacation` (`self.K2_GetActorLocation` (`local.FLActor_Rotation`))))
    (:`Is Not Valid`
      _))
  (`self.K2_SetActorLocation` (`local.FLActor_Rotation`) (+ (`local.FLacation`) (`KismetMathLibrary.RotateAngleAxis` (`KismetMathLibrary.MakeVector` (`local.FRadian`)) (+ (`local.FTaux`) (`local.FAngle`)) (0.0 0.0 1.0))) false false)
  (return (`local.FLacation`)))

(fn `UserConstructionScript`)