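; Solar system actor that animates three planets with self-rotation and orbits.
; BeginPlay runs an endless 0.1-second Delay loop instead of using Tick.
; Planet1 spins through a wrapped yaw counter, while Planet2 and Planet3 are set to a constant yaw, so they do not spin relative to their parents.
; Three Distance pivots advance yaw from their world rotation at halving rates, applied as relative rotation.
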(event `self.ReceiveBeginPlay`
  (bind _distance_planet2 (`self.distance_planet2`))
  (bind _distance_planet3 (`self.distance_planet3`))
  (bind _planet1 (`self.planet1`))
  (bind _distance_planet1 (`self.distance_planet1`))
  (bind (_returnvalue_roll _returnvalue_pitch _returnvalue_yaw) (`KismetMathLibrary.BreakRotator` (`SceneComponent.K2_GetComponentRotation` _distance_planet3)))
  (bind (_returnvalue_roll_2 _returnvalue_pitch_2 _returnvalue_yaw_2) (`KismetMathLibrary.BreakRotator` (`SceneComponent.K2_GetComponentRotation` _distance_planet1)))
  (bind (_returnvalue_roll_3 _returnvalue_pitch_3 _returnvalue_yaw_3) (`KismetMathLibrary.BreakRotator` (`SceneComponent.K2_GetComponentRotation` _distance_planet2)))
  (bind _returnvalue (+ (`self.rotation planet1`) 1.0))
  (`KismetSystemLibrary.Delay` 0.1 :!label _label)
  (if (< _returnvalue 360.0)
    (bind _output_get (set `self.rotation planet1` _returnvalue))
    (`SceneComponent.K2_SetRelativeRotation` _planet1 (`KismetMathLibrary.MakeRotator` 0.0 0.0 _output_get) false false)
    (else
      (bind _output_get_2 (set `self.rotation planet1` 0.0))
      (`SceneComponent.K2_SetRelativeRotation` _planet1 (`KismetMathLibrary.MakeRotator` 0.0 0.0 _output_get_2) false false)))
  (`SceneComponent.K2_SetRelativeRotation` (`self.planet2`) (`KismetMathLibrary.MakeRotator` 0.0 0.0 (+ 1.0 1.0)) false false)
  (`SceneComponent.K2_SetRelativeRotation` (`self.planet3`) (`KismetMathLibrary.MakeRotator` 0.0 0.0 (+ 1.0 1.0)) false false)
  (`SceneComponent.K2_SetRelativeRotation` _distance_planet1 (`KismetMathLibrary.MakeRotator` 0.0 0.0 (+ _returnvalue_yaw_2 0.125)) false false)
  (`SceneComponent.K2_SetRelativeRotation` _distance_planet2 (`KismetMathLibrary.MakeRotator` 0.0 0.0 (+ _returnvalue_yaw_3 0.0625)) false false)
  (`SceneComponent.K2_SetRelativeRotation` _distance_planet3 (`KismetMathLibrary.MakeRotator` 0.0 0.0 (+ _returnvalue_yaw 0.03125)) false false)
  (goto _label))

(event `self.ReceiveTick`
  (params (DeltaSeconds :type "Float (single-precision)")))

(fn `UserConstructionScript`)